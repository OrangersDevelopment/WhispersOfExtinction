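; BP_RangedWeaponParent is a base class for ranged weapons, handling magazine and reserve ammo, firing and reloading.
; Attack spends a round and calls the empty ShootBullet stub if the player's BP_TopDownCharacter allows firing, or reloads when the magazine is empty.
; Reloading moves ammo instantly from reserve, showing a ReloadUI widget timed by ReloadSpeed only when reserve ammo remains afterward.
; Getters expose the ammo counts and limits.
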(event EventBeginPlay
  (|CallParentFunction) ; This node is disabled and will not be called.\nDrag off pins to build functionality.
)

(event Collision|EventActorBeginOverlap
  (params (OtherActor :type Actor%20Object%20Reference))
  (|CallParentFunction OtherActor) ; This node is disabled and will not be called.\nDrag off pins to build functionality.
)

(event EventTick
  (params (DeltaSeconds :type Float%20%28single-precision%29))
  (|CallParentFunction DeltaSeconds) ; This node is disabled and will not be called.\nDrag off pins to build functionality.
)

(event EventReload
  (CallFunction|ReloadWeapon))

(event EventAttack
  (params (AnimBlueprint :type ABP%20Manny%20Object%20Reference) (Mesh :type Skeletal%20Mesh%20Component%20Object%20Reference))
  (CallFunction|FireWeapon))

(fn ConstructionScript
  (|CallParentFunction))

(fn FireWeapon
  ;[1 1 1] Fire weapon logic
  (bind _asbp_top_down_character (Utilities|Casting|CastToBP_TopDownCharacter (Game|GetPlayerCharacter 0)))
  (if (Variables|/Game/TopDown/Blueprints/BP_TopDownCharacter.BP_TopDownCharacter_C|GetCanFireWeapon _asbp_top_down_character)
    (if (> (Variables|Default|GetCurrentMagazine) 0)
      (Variables|Default|SetCurrentMagazine (- (Variables|Default|GetCurrentMagazine) 1))
      (CallFunction|ShootBullet)
      (else
        (CallFunction|ReloadWeapon)))))

(fn ReloadWeapon
  ;[1 1 1] Reloading weapon logic
  (if (> (- (Variables|Default|GetAmmo) (- (Variables|Default|GetMagazineSize) (Variables|Default|GetCurrentMagazine))) 0)
    (Variables|Default|SetAmmo (- (Variables|Default|GetAmmo) (- (Variables|Default|GetMagazineSize) (Variables|Default|GetCurrentMagazine))))
    (Variables|Default|SetCurrentMagazine (Variables|Default|GetMagazineSize))
    (CallFunction|PlayReloadAnimation)
    (else
      (Variables|Default|SetCurrentMagazine (+ (Variables|Default|GetAmmo) (Variables|Default|GetCurrentMagazine)))
      (Variables|Default|SetAmmo 0))))

(fn ShootBullet)

(fn GetCurrentMagazine
  (return (Variables|Default|GetCurrentMagazine)))

(fn GetMagazineSize
  (return (Variables|Default|GetMagazineSize)))

(fn GetAmmoMax
  (return (Variables|Default|GetMaxAmmo)))

(fn GetAmmo
  (return (Variables|Default|GetAmmo)))

(fn PlayReloadAnimation
  (bind _returnvalue (UserInterface|CreateWidget "/Game/UI/WeaponsUI/ReloadUI.ReloadUI_C" 0 (Variables|Default|GetReloadSpeed)))
  (UserInterface|Viewport|AddtoViewport _returnvalue 0))