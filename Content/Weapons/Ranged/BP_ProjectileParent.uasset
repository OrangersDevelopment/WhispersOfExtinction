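; Parent projectile Blueprint for ranged weapons that damages what it overlaps and expires after a set lifetime.
; A looping one-second timer decrements Lifetime and destroys the actor when it runs out.
; Overlaps with any actor other than OwningActor send Damage and DamageType through the I_Damageable interface.
; The projectile is not destroyed on hit, only when its lifetime ends.
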(event Custom|DecrementLifetime
  ;[1 1 1] Logic for projectile lifetime
  (bind _output_get (Variables|Default|SetLifetime (- (Variables|Default|GetLifetime) 1)))
  (if (<= _output_get 0)
    (Utilities|Time|ClearandInvalidateTimerbyHandle (stale EventBeginPlay _returnvalue))
    (Actor|DestroyActor)))

(event EventBeginPlay
  ;[1 1 1] Logic for projectile lifetime
  (bind _returnvalue (Utilities|Time|SetTimerbyEvent (delegate Custom|DecrementLifetime) 1.0 true)))

(event Collision|EventActorBeginOverlap
  (params (OtherActor :type Actor%20Object%20Reference))
  ;[1 1 1] Logic for hitting an actor -- if you want something to take damage make sure it implements I_Damageable
  (if (!= OtherActor (Variables|Default|GetOwningActor))
    (bind _asi_damageable (Utilities|Casting|CastToI_Damageable OtherActor))
    (Default|RecieveDamage _asi_damageable (Variables|Default|GetDamage) (Variables|Default|GetDamageType))))

(fn ConstructionScript)