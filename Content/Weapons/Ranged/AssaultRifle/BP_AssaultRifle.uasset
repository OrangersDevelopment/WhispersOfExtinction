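; Automatic assault rifle weapon for the top-down character, built on a parent weapon class that handles core firing and reloading.
; Attacking starts a looping AttackSpeed timer that fires through the parent unless reloading, then refreshes the holder's weapon UI.
; ShootBullet spawns BP_Bullet at the muzzle with weapon damage, owned by player 0.
; Reload plays player 0's animation, blocks firing for ReloadSpeed and calls the parent reload.
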(event Custom|StartFiring
  ;[1 1 1] Weapon is automatic so this is the style of code it uses
  (bind _returnvalue (Utilities|Time|SetTimerbyEvent (delegate Custom|FireBullet) (Variables|Default|GetAttackSpeed) true)))

(event Custom|FireBullet
  ;[1 1 1] Weapon is automatic so this is the style of code it uses
  (if (not (Variables|Default|GetReloading))
    (CallFunction|FireWeapon)
    (CallFunction|UpdateAmmoUI)))

(event Custom|StopShooting
  ;[1 1 1] Weapon is automatic so this is the style of code it uses
  (Utilities|Time|ClearandInvalidateTimerbyHandle (stale Custom|StartFiring _returnvalue)))

(event Custom|ReloadDelay
  ;[1 1 1] Weapon is automatic so this is the style of code it uses
  (Development|PrintString "Reloading...")
  (Variables|Default|SetReloading true)
  (Utilities|FlowControl|Delay (Variables|Default|GetReloadSpeed))
  (Variables|Default|SetReloading false)
  (Development|PrintString "Finished Reloading"))

(event EventBeginPlay
  (|CallParentFunction) ; This node is disabled and will not be called.\nDrag off pins to build functionality.
)

(event Collision|EventActorBeginOverlap
  (params (OtherActor :type Actor%20Object%20Reference))
  (|CallParentFunction OtherActor) ; This node is disabled and will not be called.\nDrag off pins to build functionality.
)

(event EventTick
  (params (DeltaSeconds :type Float%20%28single-precision%29))
  (|CallParentFunction DeltaSeconds) ; This node is disabled and will not be called.\nDrag off pins to build functionality.
)

(event EventReload
  ;[1 1 1] Event things
  (CallFunction|ReloadWeapon))

(event EventStartAttacking
  ;[1 1 1] Event things
  (CallFunction|StartFiring))

(event EventStopAttacking
  ;[1 1 1] Event things
  (CallFunction|StopShooting))

(fn ConstructionScript
  (|CallParentFunction))

(fn FireWeapon
  (|CallParentFunction))

(fn ShootBullet
  (bind _damage (Variables|Default|GetDamage))
  ;[1 1 1] Logic to spawn bullet
  (Game|SpawnActorfromClass "/Game/Weapons/Ranged/Projectiles/BP_Bullet.BP_Bullet_C" (Transformation|GetWorldTransform (Variables|Default|GetMuzzle)) "Undefined" "MultiplyWithRoot" 0 _damage (Variables|Default|GetDamageType) _damage (Game|GetPlayerCharacter 0) 0))

(fn GetMagazineSize
  (return (Variables|Default|GetMagazineSize)))

(fn GetCurrentMagazine
  (return (Variables|Default|GetCurrentMagazine)))

(fn GetAmmo
  (return (Variables|Default|GetAmmo)))

(fn GetAmmoMax
  (return (Variables|Default|GetMaxAmmo)))

(fn ReloadWeapon
  (bind _asbp_top_down_character (Utilities|Casting|CastToBP_TopDownCharacter (Game|Player|GetPlayerPawn 0)))
  (Default|PlayReloadAnim _asbp_top_down_character)
  (CallFunction|ReloadDelay)
  (|CallParentFunction))

(fn UpdateAmmoUI
  (bind _heldactor (Variables|Default|GetHeldActor))
  (Utilities|IsValid _heldactor
    (:Is%20Valid
      (bind _asbp_top_down_character (Utilities|Casting|CastToBP_TopDownCharacter _heldactor))
      (Default|UpdateWeaponUI _asbp_top_down_character))))

(fn GetAutomatic
  (return true))

(fn SetWeaponHolder
  (params (Actor :type Actor%20Object%20Reference))
  (bind _output_get (Variables|Default|SetHeldActor Actor))
  (return _output_get))