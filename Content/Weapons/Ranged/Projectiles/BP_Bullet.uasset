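; Bullet projectile Actor for ranged weapons that damages what it overlaps and expires after a limited lifetime.
; On BeginPlay it copies the weapon's damage and damage type, then starts a looping one-second timer that counts Lifetime down and destroys the bullet at zero.
; Overlaps with actors other than its owner send damage through the I_Damageable interface, without destroying the bullet.
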(event Custom|CustomEvent
  ;[1 1 1] Lifetime logic
  (bind _output_get (Variables|Default|SetLifetime (- (Variables|Default|GetLifetime) 1)))
  (if (<= _output_get 0)
    (Utilities|Time|ClearandInvalidateTimerbyHandle (stale EventBeginPlay _returnvalue))
    (Actor|DestroyActor)))

(event EventBeginPlay
  ;[1 1 1] Lifetime logic
  (bind _returnvalue (Utilities|Time|SetTimerbyEvent (delegate Custom|CustomEvent) 1.0 true))
  (Variables|Default|SetDamage (Variables|Default|GetWeaponDamage))
  (Variables|Default|SetDamageType (Variables|Default|GetWeaponDamageType)))

(event Collision|EventActorBeginOverlap
  (params (OtherActor :type Actor%20Object%20Reference))
  ;[1 1 1] Hitting things logic
  (if (!= OtherActor (Variables|Default|GetOwningActor))
    (bind _asi_damageable (Utilities|Casting|CastToI_Damageable OtherActor))
    (Default|RecieveDamage _asi_damageable (Variables|Default|GetDamage) (Variables|Default|GetDamageType))))

(fn ConstructionScript
  (|CallParentFunction))