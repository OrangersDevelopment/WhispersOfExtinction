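; Pistol weapon Blueprint for a top-down character, reporting itself as non-automatic.
; Attack calls FireWeapon unless a reload is in progress.
; Reload plays the player pawn's reload animation and holds a Reloading flag for a timed delay, without changing ammo counts in this graph.
; Simple functions set the holder and expose magazine and ammo values, while AddAmmo is an empty stub.
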(event EventBeginPlay
  (|CallParentFunction) ; This node is disabled and will not be called.\nDrag off pins to build functionality.
)

(event Collision|EventActorBeginOverlap
  (params (OtherActor :type Actor%20Object%20Reference))
  (|CallParentFunction OtherActor) ; This node is disabled and will not be called.\nDrag off pins to build functionality.
)

(event EventTick
  (params (DeltaSeconds :type Float%20%28single-precision%29))
  (|CallParentFunction DeltaSeconds) ; This node is disabled and will not be called.\nDrag off pins to build functionality.
)

(event EventAttack
  (params (AnimBlueprint :type ABP%20Manny%20Object%20Reference) (Mesh :type Skeletal%20Mesh%20Component%20Object%20Reference))
  (if (not (Variables|Default|GetReloading))
    (CallFunction|FireWeapon)))

(event EventReload
  (bind _asbp_top_down_character (Utilities|Casting|CastToBP_TopDownCharacter (Game|Player|GetPlayerPawn 0)))
  (Default|PlayReloadAnim _asbp_top_down_character)
  (Development|PrintString "Reloading...")
  (Variables|Default|SetReloading true)
  (Utilities|FlowControl|Delay (Variables|Default|GetReloadSpeed))
  (Variables|Default|SetReloading false)
  (Development|PrintString "Finished Reloading"))

(event EventAddAmmo)

(fn ConstructionScript
  (|CallParentFunction))

(fn SetWeaponHolder
  (params (Actor :type Actor%20Object%20Reference))
  (bind _output_get (Variables|Default|SetHeldActor Actor))
  (return _output_get))

(fn GetMagazineSize
  (return (Variables|Default|GetMagazineSize)))

(fn GetCurrentMagazine
  (return (Variables|Default|GetCurrentMagazine)))

(fn GetAutomatic
  (return false))

(fn GetAmmoMax
  (return (Variables|Default|GetMaxAmmo)))

(fn GetAmmo
  (return (Variables|Default|GetAmmo)))