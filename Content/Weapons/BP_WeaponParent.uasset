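; BP_WeaponParent is a base weapon Blueprint that defines a common interface for weapons in the game.
; Placeholder getters for ammo, max ammo, current magazine, magazine size and automatic fire return zero or false.
; SetWeaponHolder stores the holding actor in HeldActor and returns it.
; The event graph and construction script contain no logic.
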(event EventBeginPlay)

(event Collision|EventActorBeginOverlap
  (params (OtherActor :type Actor%20Object%20Reference)))

(event EventTick
  (params (DeltaSeconds :type Float%20%28single-precision%29)))

(fn ConstructionScript)

(fn GetAmmo
  (return 0))

(fn GetAmmoMax
  (return 0))

(fn GetAutomatic
  (return false))

(fn GetCurrentMagazine
  (return 0))

(fn GetMagazineSize
  (return 0))

(fn SetWeaponHolder
  (params (Actor :type Actor%20Object%20Reference))
  (bind _output_get (Variables|Default|SetHeldActor Actor))
  (return _output_get))