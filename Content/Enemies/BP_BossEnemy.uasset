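; Boss enemy that chases the player, deals melee damage and, on death, removes a door through PlayingGamemode.
; Chasing starts on BeginPlay, pawn sighting or damage, using AIMoveTo, while a looping timer also triggers close-range attacks.
; Attacks set animation flags and briefly enable DealDamageBox collision to apply ContactDamage on overlap.
; Falling below half health triggers a one-time taunt that halts movement; animation casts mix ABP_Enemy and ABP_BossEnemy.
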(event OnSeePawn(PawnSensing)
  (params (Pawn :type Pawn%20Object%20Reference))
  ;[1 1 1] See player
  (Variables|Default|SetIsSeeingPlayer true)
  (CallFunction|FollowPlayer Pawn))

(event OnComponentBeginOverlap(DealDamageBox)
  (params (OverlappedComponent :type Primitive%20Component%20Object%20Reference) (OtherActor :type Actor%20Object%20Reference) (OtherComp :type Primitive%20Component%20Object%20Reference) (OtherBodyIndex :type Integer) (bFromSweep :type Boolean) (SweepResult :type Hit%20Result%20Structure%20%28by%20ref%29))
  ;[1 1 1] Logic for dealing damage
  (if (> (Variables|Default|GetHealth) 0)
    (Variables|Default|SetOverlappedActor OtherActor)
    (bind _asbp_top_down_character (Utilities|Casting|CastToBP_TopDownCharacter (Variables|Default|GetOverlappedActor)))
    (Default|TakeDamage _asbp_top_down_character (Variables|Default|GetContactDamage))
    (Collision|SetCollisionEnabled (Variables|Default|GetDealDamageBox) "NoCollision")
    (Development|PrintString "off")))

(event Custom|Follow%20Player
  (params (EnemySpotted :type Actor%20Object%20Reference))
  (bind _returnvalue (Game|GetPlayerCharacter 0))
  (bind _dealdamagebox (Variables|Default|GetDealDamageBox))
  (bind _returnvalue_2 (Transformation|GetActorLocation _returnvalue))
  (bind _returnvalue_3 (Transformation|GetActorLocation _returnvalue))
  ;[1 1 1] Following player
  (if (Variables|Default|GetIsSeeingPlayer)
    (Utilities|IsValid _returnvalue
      (:Is%20Valid
        (AI|AIMoveTo self (Math|Vector|MakeVector (.x _returnvalue_3) (.y _returnvalue_3) (.z _returnvalue_3)) 0 1e+01 false
          (:then
            (Utilities|IsValid _returnvalue :!label _label
              (:Is%20Valid
                (AI|AIMoveTo 0 (Math|Vector|MakeVector (.x _returnvalue_2) (.y _returnvalue_2) 0.0) 0 3.0 true
                  (:then
                    (Variables|Default|SetCanAttack false))))))
          (:OnSuccess
            (Variables|Default|SetCanAttack true)
            (bind _asabp_boss_enemy (Utilities|Casting|CastToABP_BossEnemy (Components|SkeletalMesh|GetAnimInstance (Variables|Character|GetMesh))))
            (Variables|/Game/Characters/Mannequins/Animations/ABP_BossEnemy.ABP_BossEnemy_C|SetAttack _asabp_boss_enemy true)
            (AI|AIMoveTo 0 (Math|Vector|MakeVector 0.0 0.0 0.0) 0 3.0 true
              (:then
                (Utilities|FlowControl|Delay 0.5)
                (Collision|SetCollisionEnabled _dealdamagebox "QueryAndPhysics")
                (Utilities|FlowControl|Delay 0.6)
                (Collision|SetCollisionEnabled _dealdamagebox "NoCollision")
                (Variables|/Game/Characters/Mannequins/Animations/ABP_BossEnemy.ABP_BossEnemy_C|SetAttack _asabp_boss_enemy false))))
          (:OnFail
            (goto _label)))))))

(event Custom|AttackingTimer
  ;[1 1 1] Make sure will constantly attack if standing next to you
  (Utilities|Time|SetTimerbyEvent (delegate Custom|AttackPlayer) 0.2 true))

(event Custom|AttackPlayer
  (bind _dealdamagebox (Variables|Default|GetDealDamageBox))
  ;[1 1 1] Make sure will constantly attack if standing next to you
  (if (not (Variables|Default|Getattacking))
    (if (< (Math|Vector|Distance(Vector) (Transformation|GetActorLocation) (Transformation|GetActorLocation (Game|GetPlayerCharacter 0))) 5e+01)
      (Variables|Default|Setattacking true)
      (Variables|Default|SetCanAttack true)
      (bind _asabp_enemy (Utilities|Casting|CastToABP_Enemy (Components|SkeletalMesh|GetAnimInstance (Variables|Character|GetMesh))))
      (Variables|/Game/Characters/Mannequins/Animations/ABP_Enemy.ABP_Enemy_C|SetAttack _asabp_enemy true)
      (AI|AIMoveTo 0 (Math|Vector|MakeVector 0.0 0.0 0.0) 0 3.0 true
        (:then
          (Utilities|FlowControl|Delay 0.5)
          (Collision|SetCollisionEnabled _dealdamagebox "QueryAndPhysics")
          (Utilities|FlowControl|Delay 0.6)
          (Collision|SetCollisionEnabled _dealdamagebox "NoCollision")
          (Variables|/Game/Characters/Mannequins/Animations/ABP_Enemy.ABP_Enemy_C|SetAttack _asabp_enemy false)
          (Variables|Default|Setattacking false))))))

(event Custom|Taunt
  (params (AnimBP :type ABP%20Boss%20Enemy%20Object%20Reference))
  (bind _charactermovement (Variables|Character|GetCharacterMovement))
  ;[1 1 1] Taunt anim
  (Variables|/Script/Engine.CharacterMovementComponent|SetMaxWalkSpeed _charactermovement 0.0)
  (Variables|/Game/Characters/Mannequins/Animations/ABP_BossEnemy.ABP_BossEnemy_C|SetTauntEnemy AnimBP true)
  (Utilities|FlowControl|Delay 3.0)
  (Variables|/Game/Characters/Mannequins/Animations/ABP_BossEnemy.ABP_BossEnemy_C|SetTauntEnemy AnimBP false)
  (Variables|/Script/Engine.CharacterMovementComponent|SetMaxWalkSpeed _charactermovement 7e+02))

(event EventRecieveDamage
  (params (Damage :type Integer) (DamageType :type E_DamageTypes%20Enum :default "NewEnumerator0"))
  ;[1 1 1] on take damage
  (CallFunction|SpawnDamageIndicator Damage DamageType)
  (bind _output_get (Variables|Default|SetHealth (- (Variables|Default|GetHealth) Damage)))
  (if (< _output_get 0)
    (CallFunction|Die)
    (else
      (Variables|Default|SetIsSeeingPlayer true)
      (CallFunction|FollowPlayer)
      (if (< (Variables|Default|GetHealth) (/ (Variables|Default|GetMaxHealth) 2))
        (Utilities|FlowControl|DoOnce false
          (:Completed
            (bind _asabp_boss_enemy (Utilities|Casting|CastToABP_BossEnemy (Components|SkeletalMesh|GetAnimInstance (Variables|Character|GetMesh))))
            (CallFunction|Taunt _asabp_boss_enemy)))))))

(event EventBeginPlay
  ;[1 1 1] Begin play
  (Variables|Default|SetIsSeeingPlayer true)
  (CallFunction|FollowPlayer)
  (Collision|SetCollisionEnabled (Variables|Default|GetDealDamageBox) "NoCollision")
  (CallFunction|AttackingTimer))

(event EventDie
  (bind _asplaying_gamemode (Utilities|Casting|CastToPlayingGamemode (Game|GetGameMode)))
  (Default|RemoveDoor _asplaying_gamemode)
  (Default|EnemyDied _asplaying_gamemode)
  (bind _asabp_enemy (Utilities|Casting|CastToABP_Enemy (Components|SkeletalMesh|GetAnimInstance (Variables|Character|GetMesh))))
  (Variables|/Game/Characters/Mannequins/Animations/ABP_Enemy.ABP_Enemy_C|SetDead _asabp_enemy true)
  (Collision|SetCollisionEnabled (Variables|Default|GetCapsuleComponent) "PhysicsOnly")
  (Class|PawnSensingComponent|SetSensingUpdatesEnabled (Variables|Default|GetPawnSensing) false)
  (Utilities|FlowControl|Delay 4.0)
  (Actor|DestroyActor))

(fn ConstructionScript
  (|CallParentFunction))